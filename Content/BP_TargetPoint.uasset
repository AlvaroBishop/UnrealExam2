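; BP_TargetPoint is an actor that shuttles back and forth along the world X axis.
; Tick accumulates delta time and flips the IsMovingRight flag each time the timer passes five seconds, then resets it.
; Otherwise it offsets the location by one unit per frame in the current direction, without sweep, so travel distance depends on frame rate.
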(event `self.ReceiveTick`
  (params (DeltaSeconds :type "Float (single-precision)"))
  (bind _time (`self.Time`))
  (set `self.Time` (+ DeltaSeconds _time))
  (`/Engine/EditorBlueprintResources/StandardMacros.CompareFloat` _time 5.0
    (:`>`
      (if (`self.isMovingRight`)
        (set `self.isMovingRight` false)
        (else
          (set `self.isMovingRight` true)))
      (set `self.Time` 0.0))
    (:`<`
      (if (`self.isMovingRight`)
        (`self.K2_SetActorLocation` (+ (`self.K2_GetActorLocation`) (1.0 0.0 0.0)))
        (else
          (`self.K2_SetActorLocation` (+ (`self.K2_GetActorLocation`) (-1.0 -0.0 0.0))))))))

(fn `UserConstructionScript`)